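; BP_ProxLight is a proximity-detection actor that prints a debug message when the player is near and visible, with no light logic in its graphs.
; Each Tick it runs a debug-drawn Visibility line trace from its Arrow component to the player pawn.
; Detection requires the trace's blocking hit to be the pawn within MinPlayerDistance, so occluding objects prevent it.
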(event `self.ReceiveTick`
  (params (DeltaSeconds :type "Float (single-precision)"))
  (bind _outhit (`KismetSystemLibrary.LineTraceSingle` :`Start` (`SceneComponent.K2_GetComponentLocation` (`self.Arrow`)) :`End` (`self.K2_GetActorLocation` (`GameplayStatics.GetPlayerPawn` 0)) :`TraceChannel` "TraceTypeQuery1" :`DrawDebugType` "ForOneFrame"))
  (bind (_bblockinghit _binitialoverlap _time _distance _location _impactpoint _normal _impactnormal _physmat _hitactor) (`GameplayStatics.BreakHitResult` _outhit))
  (if (and _bblockinghit (<= _distance (`self.MinPlayerDistance`)) (== _hitactor (`GameplayStatics.GetPlayerPawn` 0)))
    (`KismetSystemLibrary.PrintString` "PLAYER NEAR")))

(fn `UserConstructionScript`)