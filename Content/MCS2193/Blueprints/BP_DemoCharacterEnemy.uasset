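; BP_DemoCharacterEnemy is an enemy character that senses the player and can shoot projectiles.
; PawnSensing sightings of BP_ThirdPersonCharacter write Player and SeePlayer to the AI controller's blackboard, with a retriggerable delay clearing SeePlayer shortly after the last sighting.
; Hearing noise only prints a debug message.
; Shoot plays a montage, spawns BP_Projectile at an offset along the actor's rotation and plays a laser sound, with no caller in this file.
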(event `self.PawnSensing.OnSeePawn`
  (params (Pawn :type "Pawn Object Reference"))
  (`KismetSystemLibrary.PrintString` "See Pawn")
  (`self.SetBlackBoardEnemy`)
  (bind _output_get (set `self.SensedPawn` Pawn))
  (cast `/Game/ThirdPerson/Blueprints/BP_ThirdPersonCharacter` _output_get
    (:`then`
      (`BlackboardComponent.SetValueAsObject` (`self.BlackBoardEnemy`) (`self.Player`) (`self.SensedPawn`))
      (`BlackboardComponent.SetValueAsBool` (`self.BlackBoardEnemy`) (`self.SeePlayer`) true)
      (`KismetSystemLibrary.PrintString` "SeePlayer is Set")
      (`|ExecutionSequence`
        (:`then_1`
          (`KismetSystemLibrary.RetriggerableDelay` 2.0)
          (`BlackboardComponent.SetValueAsBool` (`self.BlackBoardEnemy`) (`self.SeePlayer`) false))))
    (:`CastFailed`
      (`KismetSystemLibrary.PrintString` "Cast pawn is not the player"))))

(event `self.PawnSensing.OnHearNoise`
  (params (Instigator :type "Pawn Object Reference") (Location :type "Vector Structure (by ref)") (Volume :type "Float (single-precision)"))
  (`KismetSystemLibrary.PrintString` "Heard noise (patrol area)"))

(fn `SetBlackBoardEnemy`
  (set `self.BlackBoardEnemy` (`AIBlueprintHelperLibrary.GetBlackboard` (`AIBlueprintHelperLibrary.GetAIController` self))))

(fn `Shoot`
  (`self.PlayAnimMontage` null)
  (`|SpawnActorFromClass` "/Game/MCS2193/Blueprints/BP_Projectile.BP_Projectile_C" (`KismetMathLibrary.MakeTransform` (+ (`self.K2_GetActorLocation`) (`self.ProjectileOffset`)) (`self.K2_GetActorRotation`)) "Undefined" "MultiplyWithRoot" null null)
  (`GameplayStatics.PlaySound2D` "/Game/MCS2193/Sounds/SC_LaserShoot.SC_LaserShoot" 1.0 1.0 0.0 null null))

(fn `UserConstructionScript`)